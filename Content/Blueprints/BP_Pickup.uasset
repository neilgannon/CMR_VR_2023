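; BP_Pickup is a physics-driven static mesh actor that can be picked up and dropped.
; Pickup disables physics and attaches to the passed-in component; if its mesh has the grip socket, it attaches using that socket name with location snapped, otherwise it keeps its grab position.
; Drop detaches it in world space and re-enables physics, while Interact is an empty stub.
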(event EventInteract)

(event EventDrop
  (Transformation|DetachFromActor "KeepWorld" "KeepWorld" "KeepWorld")
  (Physics|SetSimulatePhysics (Variables|Debug|GetStaticMeshComponent) true))

(event EventPickup
  (params (AttachTo :type Scene%20Component%20Object%20Reference))
  (bind _staticmeshcomponent (Variables|Debug|GetStaticMeshComponent))
  (Physics|SetSimulatePhysics _staticmeshcomponent false)
  (if (Transformation|DoesSocketExist _staticmeshcomponent (Variables|Default|GetGripSocketName))
    ;[1 1 1] Attach to a specifc Socket added in the mesh editor
    (Transformation|AttachComponentToComponent AttachTo (Variables|Default|GetGripSocketName) "SnapToTarget" "KeepWorld" "KeepWorld" false)
    (else
      ;[1 1 1] Attach at the Grab Location
      (Transformation|AttachComponentToComponent AttachTo "None" "KeepWorld" "KeepWorld" "KeepWorld" false))))

(fn ConstructionScript)