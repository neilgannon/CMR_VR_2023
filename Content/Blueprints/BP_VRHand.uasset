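; VR hand actor that tracks a motion controller and lets the player grab, drop and use items.
; An overlap sphere detects IPIckup actors while the hand is empty, triggering haptics and storing the grab candidate.
; Grab, Drop and UseItem message the item through pickup and interactable interfaces, while Tick copies GripState to the hand animation Blueprint.
; The construction script sets the motion source from Hand and mirrors the mesh for the left.
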(event OnComponentBeginOverlap(Sphere)
  (params (OverlappedComponent :type Primitive%20Component%20Object%20Reference) (OtherActor :type Actor%20Object%20Reference) (OtherComp :type Primitive%20Component%20Object%20Reference) (OtherBodyIndex :type Integer) (bFromSweep :type Boolean) (SweepResult :type Hit%20Result%20Structure%20%28by%20ref%29))
  (if (Utilities|DoesObjectImplementInterface OtherActor "/Game/Blueprints/IPIckup.IPIckup_C")
    (if (not (Utilities|IsValid (Variables|Default|GetGrabbedActor)))
      (Class|PlayerController|PlayHapticEffect (Game|GetPlayerController 0) "/Game/Blueprints/BP_VRHandHaptic.BP_VRHandHaptic" (Variables|Default|GetHand) (Variables|Default|GetHapticScale) false)
      (Variables|Default|SetWantsToGrip? true)
      (Variables|Default|SetGripState "NewEnumerator1")
      (Variables|Default|SetAvailablePickupActor OtherActor))))

(event OnComponentEndOverlap(Sphere)
  (params (OverlappedComponent :type Primitive%20Component%20Object%20Reference) (OtherActor :type Actor%20Object%20Reference) (OtherComp :type Primitive%20Component%20Object%20Reference) (OtherBodyIndex :type Integer))
  (if (Utilities|DoesObjectImplementInterface OtherActor "/Game/Blueprints/IPIckup.IPIckup_C")
    (if (not (Utilities|IsValid (Variables|Default|GetGrabbedActor)))
      (Variables|Default|SetWantsToGrip? false)
      (Variables|Default|SetGripState "NewEnumerator0")
      (Variables|Default|SetAvailablePickupActor 0))))

(event EventTick
  (params (DeltaSeconds :type Float%20%28single-precision%29))
  ;[1 1 1] Update Animation Blueprint
  (bind _asright_hand_anim_bp (Utilities|Casting|CastToRightHand_AnimBP (Components|SkeletalMesh|GetAnimInstance (Variables|Default|GetHandMesh))))
  (Variables|/Game/Mannequin/Animations/RightHand_AnimBP.RightHand_AnimBP_C|SetGripState _asright_hand_anim_bp (Variables|Default|GetGripState)))

(fn ConstructionScript
  (bind _hand (Variables|Default|GetHand))
  (Variables|/Script/HeadMountedDisplay.MotionControllerComponent|SetMotionSource (Variables|Default|GetMotionController) (Utilities|Name|EnumtoName _hand))
  (if (Utilities|Enum|Equal(Enum) _hand "Left")
    (Transformation|SetWorldScale3D (Variables|Default|GetHandMesh) "1.000000,1.000000,-1.000000")))

(fn Grab
  (Variables|Default|SetGripState "NewEnumerator2")
  (if (Variables|Default|GetWantsToGrip?)
    (Variables|Default|GetGrabbedActor
      (:then
        (return))
      (:else
        (bind _availablepickupactor (Variables|Default|GetAvailablePickupActor)
          (:then
            (Class|IPIckup|Pickup(Message) _availablepickupactor (Variables|Default|GetMotionController))
            (Variables|Default|SetGrabbedActor _availablepickupactor)
            (Variables|Default|SetAvailablePickupActor 0))
          (:else
            (return)))))))

(fn Drop
  (Variables|Default|SetGripState "NewEnumerator0")
  (bind _grabbedactor (Variables|Default|GetGrabbedActor)
    (:then
      (Class|IPIckup|Drop(Message) _grabbedactor)
      (Variables|Default|SetGrabbedActor 0))
    (:else
      (return))))

(fn UseItem
  (bind _grabbedactor (Variables|Default|GetGrabbedActor))
  (Variables|Default|GetGrabbedActor
    (:then
      (if (Utilities|DoesObjectImplementInterface _grabbedactor "/Game/Blueprints/IInteractable.IInteractable_C")
        (Class|IInteractable|Interact(Message) _grabbedactor)))
    (:else
      (return))))